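; BP_Palo is an actor that casts a debug line trace from its Top component while the player is aiming.
; BeginPlay caches the player's BP_ThirdPersonCharacter, and Tick checks its IsAiming flag every frame.
; While aiming, it traces on the Visibility channel along Top's up vector for RaycastLength, drawing the line briefly; the hit result is unused.
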(event `self.ReceiveBeginPlay`
  (bind _asbp_third_person_character (cast `/Game/ThirdPerson/Blueprints/BP_ThirdPersonCharacter` (`GameplayStatics.GetPlayerCharacter` 0)))
  (set `self.As BP Third Person Character` _asbp_third_person_character))

(event `self.ReceiveTick`
  (params (DeltaSeconds :type "Float (single-precision)"))
  (bind _top (`self.Top`))
  (bind _returnvalue (`SceneComponent.K2_GetComponentLocation` _top))
  (if (`/Game/ThirdPerson/Blueprints/BP_ThirdPersonCharacter.IsAiming` (`self.As BP Third Person Character`))
    (`KismetSystemLibrary.LineTraceSingle` :`Start` _returnvalue :`End` (+ _returnvalue (* (`SceneComponent.GetUpVector` _top) (`self.RaycastLength`))) :`TraceChannel` "TraceTypeQuery1" :`DrawDebugType` "ForDuration" :`DrawTime` 0.2)))

(fn `UserConstructionScript`)