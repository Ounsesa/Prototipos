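; Puzzle column actor that changes to a random height when its UpdateColumn event is called.
; A player character overlapping it tells the level's BP_ColumnsController, found on BeginPlay, to update the columns and prints a debug message.
; UpdateColumn plays a timeline that lerps the cylinder's Z scale from its current value toward the new height, moving the sphere to the Scene component's location each tick.
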(event `self.ReceiveBeginPlay`
  (bind _returnvalue (`GameplayStatics.GetActorOfClass` "/Game/Blueprints/PuzzleDiego/BP_ColumnsController.BP_ColumnsController_C"))
  (set `self.ColumnController` _returnvalue))

(event `self.ReceiveActorBeginOverlap`
  (params (OtherActor :type "Actor Object Reference"))
  (cast `/Game/ThirdPerson/Blueprints/BP_ThirdPersonCharacter` OtherActor)
  (`/Game/Blueprints/PuzzleDiego/BP_ColumnsController.UpdateColumns` (`self.ColumnController`))
  (`KismetSystemLibrary.PrintString` "Hello"))

(event `self.Sphere.OnComponentBeginOverlap`
  (params (OverlappedComponent :type "PrimitiveComponent Object Reference") (OtherActor :type "Actor Object Reference") (OtherComp :type "PrimitiveComponent Object Reference") (OtherBodyIndex :type Integer) (bFromSweep :type Boolean) (SweepResult :type "HitResult Structure (by ref)")))

(event `UpdateColumn`
  (bind (_relativescale3d_x _relativescale3d_y _relativescale3d_z) (`KismetMathLibrary.BreakVector` (`SceneComponent.RelativeScale3D` (`self.Cylinder`))))
  (bind _output_get (set `self.NewHeight` (`KismetMathLibrary.RandomFloatInRange` (`self.MinHeight`) (`self.MaxHeight`))))
  (bind (_direction _columnupdate) (`Timeline|Timeline` :!via `PlayFromStart`)
    (:`Update`
      (`SceneComponent.SetRelativeScale3D` (`self.Cylinder`) (`KismetMathLibrary.MakeVector` _relativescale3d_x _relativescale3d_y (`KismetMathLibrary.Lerp` _relativescale3d_z _output_get _columnupdate)))
      (`SceneComponent.K2_SetWorldLocation` (`self.Sphere`) (`SceneComponent.K2_GetComponentLocation` (`self.Scene`)) false false))))

(fn `UserConstructionScript`)