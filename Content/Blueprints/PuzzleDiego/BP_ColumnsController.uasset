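; Puzzle controller that updates a random subset of the BP_Column actors in the level.
; On BeginPlay it gathers every BP_Column into an array.
; UpdateColumns shuffles that array and calls UpdateColumn on successive columns, using a counter checked against NumberColumnsUpdated to stop early, then resets the counter.
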(event `self.ReceiveBeginPlay`
  (bind _outactors (`GameplayStatics.GetAllActorsOfClass` "/Game/Blueprints/PuzzleDiego/BP_Column.BP_Column_C"))
  (set `self.ColumnArray` _outactors))

(event `UpdateColumns`
  (bind _columnarray (`self.ColumnArray`))
  (`KismetArrayLibrary.Array_Shuffle` _columnarray)
  (for _array_element _columnarray
    (`/Game/Blueprints/PuzzleDiego/BP_Column.UpdateColumn` _array_element)
    (bind _result (`/Engine/EditorBlueprintResources/StandardMacros.IncrementInt` (`self.ColumnsIndex`))
      (:`  `
        (if (>= _result (`self.NumberColumnsUpdated`))
          (break)))))
  (set `self.ColumnsIndex` 0))

(fn `UserConstructionScript`)